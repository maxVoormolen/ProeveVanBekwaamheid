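; Interactable serving hatch (doorgeefluik) whose flap swings open and shut when used.
; Each use fires the open event, which instantly adds a local roll rotation to the flap mesh, scaled from Rotspeed, and flips RotSide so the next use rotates it back.
; CallUse triggers that toggle and returns false, while an InteractableObjectComponent is exposed and supplies the in-use state.
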(event Custom|open
  (if (Variables|Default|GetRotSide)
    (Transformation|AddLocalRotation (Variables|Default|GetMDL_Doorgeefluik_Luik) (* (Math|Rotator|MakeRotator (Variables|Default|Getrotspeed) 0.0 0.0) 1e+01) false false)
    (Variables|Default|SetRotSide false)
    (else
      (Transformation|AddLocalRotation (Variables|Default|GetMDL_Doorgeefluik_Luik) (* (Math|Rotator|MakeRotator (Variables|Default|Getrotspeed) 0.0 0.0) -1e+01) false false)
      (Variables|Default|SetRotSide true))))

(fn ConstructionScript)

(fn CallUse
  (CallFunction|Open)
  (return false))

(fn GetInteractableObjectComponent
  (return (Variables|Default|GetInteractableObjectComponent)))

(fn IsinUse
  (return (Variables|/Game/SDT/BP/Interactables/InteractableObjectComponent.InteractableObjectComponent_C|GetisUsing (Variables|Default|GetInteractableObjectComponent))))