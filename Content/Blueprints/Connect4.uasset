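; Connect 4 board actor with a five-by-four grid of overlap components for detecting tokens, apparently an unfinished prototype.
; Every cell's begin-overlap runs one shared check of the IsPlayerToken flag, without inspecting the overlapping actor.
; When that flag is true, it sets a single board-wide HasPlayerToken flag and calls GridSearch.
; GridSearch is an empty stub whose 4InARow result is never connected, so no win detection happens.
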(event OnComponentBeginOverlap(1x1)
  (params (OverlappedComponent :type Primitive%20Component%20Object%20Reference) (OtherActor :type Actor%20Object%20Reference) (OtherComp :type Primitive%20Component%20Object%20Reference) (OtherBodyIndex :type Integer) (bFromSweep :type Boolean) (SweepResult :type Hit%20Result%20Structure%20%28by%20ref%29))
  ;[1 0.1928 0.8785] checks if its player token
  (if (Variables|Default|GetIsPlayerToken)
    (Variables|Default|SetHasPlayerToken true)
    (if (Variables|Default|GetHasPlayerToken)
      (CallFunction|GridSearch))))

(event OnComponentBeginOverlap(1x2)
  (params (OverlappedComponent :type Primitive%20Component%20Object%20Reference) (OtherActor :type Actor%20Object%20Reference) (OtherComp :type Primitive%20Component%20Object%20Reference) (OtherBodyIndex :type Integer) (bFromSweep :type Boolean) (SweepResult :type Hit%20Result%20Structure%20%28by%20ref%29))
  ;[1 0.1928 0.8785] checks if its player token
  (if (Variables|Default|GetIsPlayerToken)
    (Variables|Default|SetHasPlayerToken true)
    (if (Variables|Default|GetHasPlayerToken)
      (CallFunction|GridSearch))))

(event OnComponentBeginOverlap(5x1)
  (params (OverlappedComponent :type Primitive%20Component%20Object%20Reference) (OtherActor :type Actor%20Object%20Reference) (OtherComp :type Primitive%20Component%20Object%20Reference) (OtherBodyIndex :type Integer) (bFromSweep :type Boolean) (SweepResult :type Hit%20Result%20Structure%20%28by%20ref%29))
  ;[1 0.1928 0.8785] checks if its player token
  (if (Variables|Default|GetIsPlayerToken)
    (Variables|Default|SetHasPlayerToken true)
    (if (Variables|Default|GetHasPlayerToken)
      (CallFunction|GridSearch))))

(event OnComponentBeginOverlap(3x3)
  (params (OverlappedComponent :type Primitive%20Component%20Object%20Reference) (OtherActor :type Actor%20Object%20Reference) (OtherComp :type Primitive%20Component%20Object%20Reference) (OtherBodyIndex :type Integer) (bFromSweep :type Boolean) (SweepResult :type Hit%20Result%20Structure%20%28by%20ref%29))
  ;[1 0.1928 0.8785] checks if its player token
  (if (Variables|Default|GetIsPlayerToken)
    (Variables|Default|SetHasPlayerToken true)
    (if (Variables|Default|GetHasPlayerToken)
      (CallFunction|GridSearch))))

(event OnComponentBeginOverlap(3x2)
  (params (OverlappedComponent :type Primitive%20Component%20Object%20Reference) (OtherActor :type Actor%20Object%20Reference) (OtherComp :type Primitive%20Component%20Object%20Reference) (OtherBodyIndex :type Integer) (bFromSweep :type Boolean) (SweepResult :type Hit%20Result%20Structure%20%28by%20ref%29))
  ;[1 0.1928 0.8785] checks if its player token
  (if (Variables|Default|GetIsPlayerToken)
    (Variables|Default|SetHasPlayerToken true)
    (if (Variables|Default|GetHasPlayerToken)
      (CallFunction|GridSearch))))

(event OnComponentBeginOverlap(3x4)
  (params (OverlappedComponent :type Primitive%20Component%20Object%20Reference) (OtherActor :type Actor%20Object%20Reference) (OtherComp :type Primitive%20Component%20Object%20Reference) (OtherBodyIndex :type Integer) (bFromSweep :type Boolean) (SweepResult :type Hit%20Result%20Structure%20%28by%20ref%29))
  ;[1 0.1928 0.8785] checks if its player token
  (if (Variables|Default|GetIsPlayerToken)
    (Variables|Default|SetHasPlayerToken true)
    (if (Variables|Default|GetHasPlayerToken)
      (CallFunction|GridSearch))))

(event OnComponentBeginOverlap(4x3)
  (params (OverlappedComponent :type Primitive%20Component%20Object%20Reference) (OtherActor :type Actor%20Object%20Reference) (OtherComp :type Primitive%20Component%20Object%20Reference) (OtherBodyIndex :type Integer) (bFromSweep :type Boolean) (SweepResult :type Hit%20Result%20Structure%20%28by%20ref%29))
  ;[1 0.1928 0.8785] checks if its player token
  (if (Variables|Default|GetIsPlayerToken)
    (Variables|Default|SetHasPlayerToken true)
    (if (Variables|Default|GetHasPlayerToken)
      (CallFunction|GridSearch))))

(event OnComponentBeginOverlap(4x2)
  (params (OverlappedComponent :type Primitive%20Component%20Object%20Reference) (OtherActor :type Actor%20Object%20Reference) (OtherComp :type Primitive%20Component%20Object%20Reference) (OtherBodyIndex :type Integer) (bFromSweep :type Boolean) (SweepResult :type Hit%20Result%20Structure%20%28by%20ref%29))
  ;[1 0.1928 0.8785] checks if its player token
  (if (Variables|Default|GetIsPlayerToken)
    (Variables|Default|SetHasPlayerToken true)
    (if (Variables|Default|GetHasPlayerToken)
      (CallFunction|GridSearch))))

(event OnComponentBeginOverlap(4x4)
  (params (OverlappedComponent :type Primitive%20Component%20Object%20Reference) (OtherActor :type Actor%20Object%20Reference) (OtherComp :type Primitive%20Component%20Object%20Reference) (OtherBodyIndex :type Integer) (bFromSweep :type Boolean) (SweepResult :type Hit%20Result%20Structure%20%28by%20ref%29))
  ;[1 0.1928 0.8785] checks if its player token
  (if (Variables|Default|GetIsPlayerToken)
    (Variables|Default|SetHasPlayerToken true)
    (if (Variables|Default|GetHasPlayerToken)
      (CallFunction|GridSearch))))

(event OnComponentBeginOverlap(5x3)
  (params (OverlappedComponent :type Primitive%20Component%20Object%20Reference) (OtherActor :type Actor%20Object%20Reference) (OtherComp :type Primitive%20Component%20Object%20Reference) (OtherBodyIndex :type Integer) (bFromSweep :type Boolean) (SweepResult :type Hit%20Result%20Structure%20%28by%20ref%29))
  ;[1 0.1928 0.8785] checks if its player token
  (if (Variables|Default|GetIsPlayerToken)
    (Variables|Default|SetHasPlayerToken true)
    (if (Variables|Default|GetHasPlayerToken)
      (CallFunction|GridSearch))))

(event OnComponentBeginOverlap(5x2)
  (params (OverlappedComponent :type Primitive%20Component%20Object%20Reference) (OtherActor :type Actor%20Object%20Reference) (OtherComp :type Primitive%20Component%20Object%20Reference) (OtherBodyIndex :type Integer) (bFromSweep :type Boolean) (SweepResult :type Hit%20Result%20Structure%20%28by%20ref%29))
  ;[1 0.1928 0.8785] checks if its player token
  (if (Variables|Default|GetIsPlayerToken)
    (Variables|Default|SetHasPlayerToken true)
    (if (Variables|Default|GetHasPlayerToken)
      (CallFunction|GridSearch))))

(event OnComponentBeginOverlap(5x4)
  (params (OverlappedComponent :type Primitive%20Component%20Object%20Reference) (OtherActor :type Actor%20Object%20Reference) (OtherComp :type Primitive%20Component%20Object%20Reference) (OtherBodyIndex :type Integer) (bFromSweep :type Boolean) (SweepResult :type Hit%20Result%20Structure%20%28by%20ref%29))
  ;[1 0.1928 0.8785] checks if its player token
  (if (Variables|Default|GetIsPlayerToken)
    (Variables|Default|SetHasPlayerToken true)
    (if (Variables|Default|GetHasPlayerToken)
      (CallFunction|GridSearch))))

(event OnComponentBeginOverlap(1x3)
  (params (OverlappedComponent :type Primitive%20Component%20Object%20Reference) (OtherActor :type Actor%20Object%20Reference) (OtherComp :type Primitive%20Component%20Object%20Reference) (OtherBodyIndex :type Integer) (bFromSweep :type Boolean) (SweepResult :type Hit%20Result%20Structure%20%28by%20ref%29))
  ;[1 0.1928 0.8785] checks if its player token
  (if (Variables|Default|GetIsPlayerToken)
    (Variables|Default|SetHasPlayerToken true)
    (if (Variables|Default|GetHasPlayerToken)
      (CallFunction|GridSearch))))

(event OnComponentBeginOverlap(1x4)
  (params (OverlappedComponent :type Primitive%20Component%20Object%20Reference) (OtherActor :type Actor%20Object%20Reference) (OtherComp :type Primitive%20Component%20Object%20Reference) (OtherBodyIndex :type Integer) (bFromSweep :type Boolean) (SweepResult :type Hit%20Result%20Structure%20%28by%20ref%29))
  ;[1 0.1928 0.8785] checks if its player token
  (if (Variables|Default|GetIsPlayerToken)
    (Variables|Default|SetHasPlayerToken true)
    (if (Variables|Default|GetHasPlayerToken)
      (CallFunction|GridSearch))))

(event OnComponentBeginOverlap(2x1)
  (params (OverlappedComponent :type Primitive%20Component%20Object%20Reference) (OtherActor :type Actor%20Object%20Reference) (OtherComp :type Primitive%20Component%20Object%20Reference) (OtherBodyIndex :type Integer) (bFromSweep :type Boolean) (SweepResult :type Hit%20Result%20Structure%20%28by%20ref%29))
  ;[1 0.1928 0.8785] checks if its player token
  (if (Variables|Default|GetIsPlayerToken)
    (Variables|Default|SetHasPlayerToken true)
    (if (Variables|Default|GetHasPlayerToken)
      (CallFunction|GridSearch))))

(event OnComponentBeginOverlap(2x3)
  (params (OverlappedComponent :type Primitive%20Component%20Object%20Reference) (OtherActor :type Actor%20Object%20Reference) (OtherComp :type Primitive%20Component%20Object%20Reference) (OtherBodyIndex :type Integer) (bFromSweep :type Boolean) (SweepResult :type Hit%20Result%20Structure%20%28by%20ref%29))
  ;[1 0.1928 0.8785] checks if its player token
  (if (Variables|Default|GetIsPlayerToken)
    (Variables|Default|SetHasPlayerToken true)
    (if (Variables|Default|GetHasPlayerToken)
      (CallFunction|GridSearch))))

(event OnComponentBeginOverlap(2x2)
  (params (OverlappedComponent :type Primitive%20Component%20Object%20Reference) (OtherActor :type Actor%20Object%20Reference) (OtherComp :type Primitive%20Component%20Object%20Reference) (OtherBodyIndex :type Integer) (bFromSweep :type Boolean) (SweepResult :type Hit%20Result%20Structure%20%28by%20ref%29))
  ;[1 0.1928 0.8785] checks if its player token
  (if (Variables|Default|GetIsPlayerToken)
    (Variables|Default|SetHasPlayerToken true)
    (if (Variables|Default|GetHasPlayerToken)
      (CallFunction|GridSearch))))

(event OnComponentBeginOverlap(2x4)
  (params (OverlappedComponent :type Primitive%20Component%20Object%20Reference) (OtherActor :type Actor%20Object%20Reference) (OtherComp :type Primitive%20Component%20Object%20Reference) (OtherBodyIndex :type Integer) (bFromSweep :type Boolean) (SweepResult :type Hit%20Result%20Structure%20%28by%20ref%29))
  ;[1 0.1928 0.8785] checks if its player token
  (if (Variables|Default|GetIsPlayerToken)
    (Variables|Default|SetHasPlayerToken true)
    (if (Variables|Default|GetHasPlayerToken)
      (CallFunction|GridSearch))))

(event OnComponentBeginOverlap(3x1)
  (params (OverlappedComponent :type Primitive%20Component%20Object%20Reference) (OtherActor :type Actor%20Object%20Reference) (OtherComp :type Primitive%20Component%20Object%20Reference) (OtherBodyIndex :type Integer) (bFromSweep :type Boolean) (SweepResult :type Hit%20Result%20Structure%20%28by%20ref%29))
  ;[1 0.1928 0.8785] checks if its player token
  (if (Variables|Default|GetIsPlayerToken)
    (Variables|Default|SetHasPlayerToken true)
    (if (Variables|Default|GetHasPlayerToken)
      (CallFunction|GridSearch))))

(event OnComponentBeginOverlap(4x1)
  (params (OverlappedComponent :type Primitive%20Component%20Object%20Reference) (OtherActor :type Actor%20Object%20Reference) (OtherComp :type Primitive%20Component%20Object%20Reference) (OtherBodyIndex :type Integer) (bFromSweep :type Boolean) (SweepResult :type Hit%20Result%20Structure%20%28by%20ref%29))
  ;[1 0.1928 0.8785] checks if its player token
  (if (Variables|Default|GetIsPlayerToken)
    (Variables|Default|SetHasPlayerToken true)
    (if (Variables|Default|GetHasPlayerToken)
      (CallFunction|GridSearch))))

(event EventBeginPlay)

(event Collision|EventActorBeginOverlap
  (params (OtherActor :type Actor%20Object%20Reference)))

(event EventTick
  (params (DeltaSeconds :type Float%20%28single-precision%29)))

(fn ConstructionScript)

(fn GridSearch)