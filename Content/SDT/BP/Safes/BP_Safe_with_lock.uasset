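; Lockable safe Blueprint whose door animation plays only once its puzzle lock is released.
; It overrides the parent's door animation, calling it only when UnlockableDoorListenerComponent reports unlocked.
; On BeginPlay it binds that component's puzzle event.
; Functions for adding puzzles and checking whether all are solved delegate to the component, which is also exposed through a getter.
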(event EventBeginPlay
  (|CallParentFunction)
  (|BindToPuzzleToThisDoor))

(event Collision|EventActorBeginOverlap
  (params (OtherActor :type Actor%20Object%20Reference))
  (|CallParentFunction OtherActor))

(event EventTick
  (params (DeltaSeconds :type Float%20%28single-precision%29))
  (|CallParentFunction DeltaSeconds))

(fn ConstructionScript
  (|CallParentFunction))

(fn PlayDoorAnimation
  (params (slide :type Float%20%28single-precision%29))
  (if (Variables|/Game/SDT/BP/Doors/Components/UnlockableDoorListenerComponent.UnlockableDoorListenerComponent_C|GetisUnlocked (Variables|Default|GetUnlockableDoorListenerComponent))
    (|CallParentFunction slide)))

(fn AddPuzzle
  (params (puzzle :type Puzzle%20Interface))
  (bind _added (Default|AddPuzzle (Variables|Default|GetUnlockableDoorListenerComponent) puzzle))
  (return _added))

(fn AreAllPuzzlesSolved
  (bind _solved (Default|AreAllPuzzlesSolved (Variables|Default|GetUnlockableDoorListenerComponent)))
  (return _solved))

(fn GetUnlockableDoorListenerComponent
  (return (Variables|Default|GetUnlockableDoorListenerComponent)))