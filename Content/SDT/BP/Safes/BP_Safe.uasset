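; BP_Safe is an interactable safe whose door swings open and closed when used.
; CallUse fires the Use event, which toggles IsClosed and plays or reverses the Slide timeline.
; Timeline updates drive PlayDoorAnimation, a separate overridable function that lerps SafeDoor's relative rotation between two rotators along the shortest path.
; It also exposes its InteractableObjectComponent and that component's IsUsing state through getter functions.
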(event EventBeginPlay)

(event Collision|EventActorBeginOverlap
  (params (OtherActor :type Actor%20Object%20Reference)))

(event EventTick
  (params (DeltaSeconds :type Float%20%28single-precision%29)))

(fn ConstructionScript)

(fn PlayDoorAnimation
  (params (slide :type Float%20%28single-precision%29))
  (Transformation|SetRelativeRotation (Variables|Default|GetSafe_Door) (Math|Rotator|Lerp(Rotator) (Variables|Default|GetcurrentDoorRotation) (LocalVariables|GetnewDoorRotation) slide true) false false))

(fn CallUse
  (CallFunction|Use)
  (return true))

(event Custom|Use
  (if (Variables|Default|GetisClosed)
    (Variables|Default|SetisClosed false)
    (bind _slide (Timeline|Slide Play)
      (:Update
        (CallFunction|PlayDoorAnimation _slide) ; Logic for opening doors is kept inside a seperate function for overridability.
      ))
    (else
      (Variables|Default|SetisClosed true)
      (Timeline|Slide Reverse))))

(fn GetInteractableObjectComponent
  (return (Variables|Default|GetInteractableObjectComponent)))

(fn IsinUse
  (return (Variables|/Game/SDT/BP/Interactables/InteractableObjectComponent.InteractableObjectComponent_C|GetisUsing (Variables|Default|GetInteractableObjectComponent))))