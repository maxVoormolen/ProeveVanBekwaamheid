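; Interactable pass-through hatch that swings between two rotations when used and can hold one grabbable object.
; CallUse triggers Open, which flips RotSide to play or reverse the Slide timeline, lerping the hatch mesh's relative rotation along the shortest path.
; A grabbable overlapping the mesh snaps to its first socket if the mesh has no attached children, which serves as the holding-item check.
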(event Custom|open
  (if (Variables|Default|GetRotSide)
    (Variables|Default|SetRotSide false)
    (bind _slide (Timeline|slide Play)
      (:Update
        (CallFunction|PlayAnimation _slide)))
    (else
      (Variables|Default|SetRotSide true)
      (Timeline|slide Reverse))))

(fn ConstructionScript)

(fn PlayAnimation
  (params (slide :type Float%20%28single-precision%29))
  (Transformation|SetRelativeRotation (Variables|Default|GetMDL_Doorgeefluik_Luik) (Math|Rotator|Lerp(Rotator) (Variables|Default|GetcurrentRotation) (LocalVariables|GetnewRotation) slide true) false false))

(fn CallUse
  (CallFunction|Open)
  (return true))

(event OnComponentBeginOverlap(MDL_Doorgeefluik_Luik)
  (params (OverlappedComponent :type Primitive%20Component%20Object%20Reference) (OtherActor :type Actor%20Object%20Reference) (OtherComp :type Primitive%20Component%20Object%20Reference) (OtherBodyIndex :type Integer) (bFromSweep :type Boolean) (SweepResult :type Hit%20Result%20Structure%20%28by%20ref%29))
  (bind (_asgrabbable_object _bsuccess) (Utilities|Casting|CastToGrabbableObject OtherActor))
  (bind _mdl_doorgeefluik_luik (Variables|Default|GetMDL_Doorgeefluik_Luik))
  ;[0.67 0.8099 1] Check if it's holding item
  (bind _isholding (CallFunction|IsHoldingItem))
  (if (and (not _isholding) _bsuccess)
    (bind _object (Default|AsActorObject _asgrabbable_object))
    (bind _name (CallFunction|GetSocketName _mdl_doorgeefluik_luik))
    (Transformation|AttachComponentToComponent _object _mdl_doorgeefluik_luik _name "SnapToTarget" "SnapToTarget" "KeepWorld" true)))

(fn GetInteractableObjectComponent
  (return (Variables|Default|GetInteractableObjectComponent)))

(fn GetSocketName
  (params (component :type Scene%20Component%20Object%20Reference%20%28by%20ref%29) (index :type Integer))
  (bind _returnvalue (Transformation|GetAllSocketNames component))
  (if (< index (Utilities|Array|Length _returnvalue))
    (LocalVariables|SetnewName (Utilities|Array|Get(acopy) _returnvalue index)))
  (return (LocalVariables|GetnewName)))

(fn IsHoldingItem
  (return (> (Utilities|Array|Length (Components|GetChildrenComponents (Variables|Default|GetMDL_Doorgeefluik_Luik) false)) 0)))

(fn IsinUse
  (return (Variables|/Game/SDT/BP/Interactables/InteractableObjectComponent.InteractableObjectComponent_C|GetisUsing (Variables|Default|GetInteractableObjectComponent))))