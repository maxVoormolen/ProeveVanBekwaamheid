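; BP_KeyPad_DoorLock is a keypad child Blueprint that unlocks a door when its puzzle succeeds.
; Its success-state override runs the parent behavior, then calls CallUnlockDoor on its PuzzleEventComponent.
; Unlock sets IsPassed and triggers that success state, while accessor functions expose the component and completion flag.
; BeginPlay, overlap, Tick and construction only forward to the parent.
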(event EventBeginPlay
  (|CallParentFunction))

(event Collision|EventActorBeginOverlap
  (params (OtherActor :type Actor%20Object%20Reference))
  (|CallParentFunction OtherActor))

(event EventTick
  (params (DeltaSeconds :type Float%20%28single-precision%29))
  (|CallParentFunction DeltaSeconds))

(fn ConstructionScript
  (|CallParentFunction))

(fn ShowSuccessState
  (|CallParentFunction)
  (Default|CallUnlockDoor (Variables|Default|GetPuzzleEventComponent)))

(fn GetPuzzleEventComponent
  (return (Variables|Default|GetPuzzleEventComponent)))

(fn IsCompleted
  (return (Variables|Default|GetIsPassed)))

(fn Unlock
  (bind _output_get (Variables|Default|SetIsPassed true))
  (CallFunction|ShowSuccessState)
  (return _output_get))