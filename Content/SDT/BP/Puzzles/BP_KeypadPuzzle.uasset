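; Keypad puzzle actor, currently a stub with no code entry or validation logic.
; Clicking the Key_0 component prints that component's object name as debug output.
; IsCompleted always returns true, so the puzzle reports itself solved regardless of input.
; BeginPlay, overlap, Tick and construction only forward to the parent class.
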(event OnClicked(key_0)
  (params (TouchedComponent :type Primitive%20Component%20Object%20Reference) (ButtonPressed :type Key%20Structure :default "None"))
  (Development|PrintString (Utilities|GetObjectName TouchedComponent) true true "(R=0.790000,G=0.987483,B=1.000000,A=1.000000)" 1.0))

(event EventBeginPlay
  (|CallParentFunction))

(event Collision|EventActorBeginOverlap
  (params (OtherActor :type Actor%20Object%20Reference))
  (|CallParentFunction OtherActor))

(event EventTick
  (params (DeltaSeconds :type Float%20%28single-precision%29))
  (|CallParentFunction DeltaSeconds))

(fn ConstructionScript
  (|CallParentFunction))

(fn IsCompleted
  (return true))